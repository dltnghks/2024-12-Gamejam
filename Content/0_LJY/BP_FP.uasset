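; BP_FP is a player-controlled Blueprint that turns its controller's view to fixed yaw angles on key presses.
; Pressing D or A plays a timeline that blends control yaw toward 90 or 0 degrees respectively, zeroing pitch and roll.
; Each update lerps from the current yaw rather than a stored start value, so the targets are absolute and the easing compounds.
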(event `Key|D`
  (params (Key :type "Key Structure"))
  (:`Pressed`
    (bind (_direction _yawprogress) (`Timeline|90degreeYaw` :!via `PlayFromStart`)
      (:`Update`
        (`Controller.SetControlRotation` (`self.GetController`) (`KismetMathLibrary.MakeRotator` 0.0 0.0 (`KismetMathLibrary.Lerp` (.yaw (`self.GetControlRotation`)) (+ 0.0 90.0) _yawprogress)))))))

(event `Key|A`
  (params (Key :type "Key Structure"))
  (:`Pressed`
    (bind (_direction _yawprogress) (`Timeline|타임라인` :!via `PlayFromStart`)
      (:`Update`
        (`Controller.SetControlRotation` (`self.GetController`) (`KismetMathLibrary.MakeRotator` 0.0 0.0 (`KismetMathLibrary.Lerp` (.yaw (`self.GetControlRotation`)) (+ 0.0 0.0) _yawprogress)))))))

(fn `UserConstructionScript`)