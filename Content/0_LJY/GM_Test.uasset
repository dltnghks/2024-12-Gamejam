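; Test game mode that spawns the first-person pawn BP_FP at a PlayerStart on BeginPlay and has the first player controller possess it.
; A PlayIntro event creates the WBP_ConversationUI widget, gathers every row of IntroDataTable into DialogList and passes that list to the widget.
; The only PlayIntro call here sits in disconnected nodes, so this graph never starts the intro itself.
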(event `self.ReceiveBeginPlay`
  (`KismetSystemLibrary.PrintString` "Hello")
  (bind _returnvalue (`GameplayStatics.GetActorOfClass` "/Script/Engine.PlayerStart"))
  (bind _returnvalue_2 (`|SpawnActorFromClass` "/Game/0_LJY/BP_FP.BP_FP_C" (`self.GetTransform` _returnvalue) "AlwaysSpawn" "MultiplyWithRoot" null null))
  (`Controller.Possess` (`GameplayStatics.GetPlayerController` 0) _returnvalue_2))

(event `PlayIntro`
  (bind _dialog_list (`self.Dialog List`))
  (bind _intro_data_table (`self.Intro Data Table`))
  (bind _returnvalue (`|CreateWidget` "/Game/Blueprints/DialogSystem/WBP_ConversationUI.WBP_ConversationUI_C" (`GameplayStatics.GetPlayerController` 0)))
  (`UserWidget.AddToViewport` _returnvalue 0)
  (bind _outrownames (`DataTableFunctionLibrary.GetDataTableRowNames` _intro_data_table))
  (for _array_element _outrownames
    (bind _returnvalue_2 (`|GetDataTableRow` _intro_data_table _array_element)
      (:`then`
        (`KismetArrayLibrary.Array_Add` _dialog_list _returnvalue_2))))
  (`/Game/Blueprints/DialogSystem/WBP_ConversationUI.SetDialogDataList` _returnvalue _dialog_list))

(fn `UserConstructionScript`)