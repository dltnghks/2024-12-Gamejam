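; BP_NPCBase is an NPC base Blueprint with two widget components, hidden at BeginPlay, that flash as left and right scare effects.
; ScareLeft and ScareRight each toggle their own widget through a delayed loop capped at 20 passes by a DoN that is never reset.
; The random delay uses integer division before conversion, so each wait is zero or one second, mostly zero.
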(event `self.ReceiveBeginPlay`
  (`SceneComponent.SetVisibility` (`self.Widget`) false false)
  (`SceneComponent.SetVisibility` (`self.Widget1`) false false))

(event `ScareLeft`
  (bind _widget (`self.Widget`))
  (`/Engine/EditorBlueprintResources/StandardMacros.Do N` 20 :!label _label
    (:`Exit`
      (`KismetSystemLibrary.Delay` (`KismetMathLibrary.Conv_IntToDouble` (/ (`KismetMathLibrary.RandomIntegerInRange` 5 10) 10)))
      (`SceneComponent.SetVisibility` _widget (not (`SceneComponent.bVisible` _widget)) false)
      (goto _label))))

(event `ScareRight`
  (bind _widget1 (`self.Widget1`))
  (`/Engine/EditorBlueprintResources/StandardMacros.Do N` 20 :!label _label_2
    (:`Exit`
      (`KismetSystemLibrary.Delay` (`KismetMathLibrary.Conv_IntToDouble` (/ (`KismetMathLibrary.RandomIntegerInRange` 5 10) 10)))
      (`SceneComponent.SetVisibility` _widget1 (not (`SceneComponent.bVisible` _widget1)) false)
      (goto _label_2))))

(fn `UserConstructionScript`)