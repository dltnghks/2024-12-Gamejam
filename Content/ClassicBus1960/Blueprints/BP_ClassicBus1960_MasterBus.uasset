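; Configurable 1960s classic bus actor with animated folding doors, switchable details and optional rolling wheels.
; The construction script poses doors, removes unused parts and drives dynamic materials for paint, dirt, rust, attrition and lights.
; Tick spins split wheels when Roll is non-zero.
; Timeline events open and close both door sets; one second after opening, the bus triggers scare events on BP_NPC01.
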(event `self.ReceiveBeginPlay`)

(event `self.ReceiveTick`
  (params (DeltaSeconds :type "Float (single-precision)"))
  (if (and (!= (`self.Roll`) 0.0) (`self.WheelsSplit`))
    (`self.WheelRoll`)))

(event `OpenDoorSmooth`
  (bind (_direction _opentrack) (`Timeline|OpenDoorTimeline` :!via `PlayFromStart`)
    (:`Update`
      (`self.FDoorAction` _opentrack)
      (`self.BDoorAction` _opentrack))
    (:`Finished`
      (`KismetSystemLibrary.Delay` 1.0)
      (bind _returnvalue (`GameplayStatics.GetActorOfClass` "/Game/Blueprints/NPC/BP_NPC01.BP_NPC01_C"))
      (bind _asbp_npc01 (cast `/Game/Blueprints/NPC/BP_NPC01` _returnvalue))
      (`/Game/Blueprints/NPC/BP_NPCBase.Scare` _asbp_npc01)
      (`/Game/Blueprints/NPC/BP_NPCBase.ScareRight` _asbp_npc01))))

(event `CloseDoorSmooth`
  (bind (_direction _closetrack) (`Timeline|CloseDoorTimeline` :!via `PlayFromStart`)
    (:`Update`
      (`self.FDoorAction` _closetrack)
      (`self.BDoorAction` _closetrack))))

(fn `BDoorAction`
  (params (Door :type "Float (double-precision)"))
  (`SceneComponent.K2_SetRelativeRotation` (`self.sm_Door_b1`) (`KismetMathLibrary.MakeRotator` 0.0 0.0 (* -90.0 Door)) false false)
  (`SceneComponent.K2_SetRelativeRotation` (`self.sm_Door_b2`) (`KismetMathLibrary.MakeRotator` 0.0 0.0 (* 180.0 Door)) false false)
  (`SceneComponent.K2_SetRelativeRotation` (`self.sm_Door_b3`) (`KismetMathLibrary.MakeRotator` 0.0 0.0 (* -180.0 Door)) false false)
  (`SceneComponent.K2_SetRelativeRotation` (`self.sm_Door_b4`) (`KismetMathLibrary.MakeRotator` 0.0 0.0 (* 90.0 Door)) false false)
  (return))

(fn `CreateDynamicMat`
  (bind _sm_curtain (`self.sm_Curtain`))
  (bind _sm_body (`self.sm_Body`))
  (bind _sm_wheels (`self.sm_Wheels`))
  (bind _sm_inside (`self.sm_Inside`))
  (bind _sm_under (`self.sm_Under`))
  (bind _sm_door_f4 (`self.sm_Door_f4`))
  (bind _sm_topdetal (`self.sm_TopDetal`))
  (bind _returnvalue (`PrimitiveComponent.CreateDynamicMaterialInstance` _sm_body 0 (`PrimitiveComponent.GetMaterial` _sm_body 0) "None"))
  (set `self.DM_body` _returnvalue)
  (bind _returnvalue_2 (`PrimitiveComponent.CreateDynamicMaterialInstance` _sm_body 1 (`PrimitiveComponent.GetMaterial` _sm_body 1) "None"))
  (set `self.DM_glass` _returnvalue_2)
  (bind _returnvalue_3 (`PrimitiveComponent.CreateDynamicMaterialInstance` _sm_body 2 (`PrimitiveComponent.GetMaterial` _sm_body 2) "None"))
  (set `self.DM_glassIN` _returnvalue_3)
  (bind _returnvalue_4 (`PrimitiveComponent.CreateDynamicMaterialInstance` _sm_wheels 0 "/Game/ClassicBus1960/Materials/IN_ClassicBus1960_backWheels.IN_ClassicBus1960_backWheels" "None"))
  (set `self.DM_BWheel` _returnvalue_4)
  (bind _returnvalue_5 (`PrimitiveComponent.CreateDynamicMaterialInstance` _sm_wheels 1 "/Game/ClassicBus1960/Materials/IN_ClassicBus1960_FrontWheels.IN_ClassicBus1960_FrontWheels" "None"))
  (set `self.DM_FWheel` _returnvalue_5)
  (bind _returnvalue_6 (`PrimitiveComponent.CreateDynamicMaterialInstance` _sm_inside 0 (`PrimitiveComponent.GetMaterial` _sm_inside 0) "None"))
  (set `self.DM_Inside` _returnvalue_6)
  (bind _returnvalue_7 (`PrimitiveComponent.CreateDynamicMaterialInstance` _sm_under 0 (`PrimitiveComponent.GetMaterial` _sm_under 0) "None"))
  (set `self.DM_Under` _returnvalue_7)
  (`PrimitiveComponent.SetMaterial` _sm_door_f4 0 (`self.DM_body`))
  (`PrimitiveComponent.SetMaterial` (`self.sm_Door_f3`) 0 (`self.DM_body`))
  (`PrimitiveComponent.SetMaterial` (`self.sm_Door_b1`) 0 (`self.DM_body`))
  (`PrimitiveComponent.SetMaterial` (`self.sm_Door_b2`) 0 (`self.DM_body`))
  (`PrimitiveComponent.SetMaterial` (`self.sm_Door_b4`) 0 (`self.DM_body`))
  (`PrimitiveComponent.SetMaterial` (`self.sm_Door_b3`) 0 (`self.DM_body`))
  (`PrimitiveComponent.SetMaterial` (`self.sm_Door_f1`) 0 (`self.DM_body`))
  (`PrimitiveComponent.SetMaterial` (`self.sm_Door_f2`) 0 (`self.DM_body`))
  (`PrimitiveComponent.SetMaterial` _sm_door_f4 1 (`self.DM_glass`))
  (`PrimitiveComponent.SetMaterial` (`self.sm_Door_f3`) 1 (`self.DM_glass`))
  (`PrimitiveComponent.SetMaterial` (`self.sm_Door_b1`) 1 (`self.DM_glass`))
  (`PrimitiveComponent.SetMaterial` (`self.sm_Door_b2`) 1 (`self.DM_glass`))
  (`PrimitiveComponent.SetMaterial` (`self.sm_Door_b4`) 1 (`self.DM_glass`))
  (`PrimitiveComponent.SetMaterial` (`self.sm_Door_b3`) 1 (`self.DM_glass`))
  (`PrimitiveComponent.SetMaterial` (`self.sm_Door_f1`) 1 (`self.DM_glass`))
  (`PrimitiveComponent.SetMaterial` (`self.sm_Door_f2`) 1 (`self.DM_glass`))
  (`PrimitiveComponent.SetMaterial` _sm_door_f4 2 (`self.DM_glassIN`))
  (`PrimitiveComponent.SetMaterial` (`self.sm_Door_f3`) 2 (`self.DM_glassIN`))
  (`PrimitiveComponent.SetMaterial` (`self.sm_Door_b1`) 2 (`self.DM_glassIN`))
  (`PrimitiveComponent.SetMaterial` (`self.sm_Door_b2`) 2 (`self.DM_glassIN`))
  (`PrimitiveComponent.SetMaterial` (`self.sm_Door_b4`) 2 (`self.DM_glassIN`))
  (`PrimitiveComponent.SetMaterial` (`self.sm_Door_b3`) 2 (`self.DM_glassIN`))
  (`PrimitiveComponent.SetMaterial` (`self.sm_Door_f1`) 2 (`self.DM_glassIN`))
  (`PrimitiveComponent.SetMaterial` (`self.sm_Door_f2`) 2 (`self.DM_glassIN`))
  (if (`self.Top`)
    (bind _returnvalue_8 (`PrimitiveComponent.CreateDynamicMaterialInstance` _sm_topdetal 0 (`PrimitiveComponent.GetMaterial` _sm_topdetal 0) "None"))
    (set `self.DM_topDetal` _returnvalue_8))
  (if (`self.Curtain`)
    (bind _returnvalue_9 (`PrimitiveComponent.CreateDynamicMaterialInstance` _sm_curtain 0 (`PrimitiveComponent.GetMaterial` _sm_curtain 0) "None"))
    (set `self.DM_Curtain` _returnvalue_9))
  (`PrimitiveComponent.SetMaterial` (`self.fw1`) 0 (`self.DM_FWheel`))
  (`PrimitiveComponent.SetMaterial` (`self.fw2`) 0 (`self.DM_FWheel`))
  (`PrimitiveComponent.SetMaterial` (`self.bw1`) 0 (`self.DM_BWheel`))
  (`PrimitiveComponent.SetMaterial` (`self.bw2`) 0 (`self.DM_BWheel`))
  (return))

(fn `DetalsSetup`
  (if (not (`self.Top`))
    (`ActorComponent.K2_DestroyComponent` (`self.sm_TopDetal`)))
  (if (`self.Curtain`)
    (return)
    (else
      (`ActorComponent.K2_DestroyComponent` (`self.sm_Curtain`))
      (return))))

(fn `FDoorAction`
  (params (Door :type "Float (double-precision)"))
  (`SceneComponent.K2_SetRelativeRotation` (`self.sm_Door_f1`) (`KismetMathLibrary.MakeRotator` 0.0 0.0 (* -90.0 Door)) false false)
  (`SceneComponent.K2_SetRelativeRotation` (`self.sm_Door_f2`) (`KismetMathLibrary.MakeRotator` 0.0 0.0 (* 180.0 Door)) false false)
  (`SceneComponent.K2_SetRelativeRotation` (`self.sm_Door_f3`) (`KismetMathLibrary.MakeRotator` 0.0 0.0 (* -180.0 Door)) false false)
  (`SceneComponent.K2_SetRelativeRotation` (`self.sm_Door_f4`) (`KismetMathLibrary.MakeRotator` 0.0 0.0 (* 90.0 Door)) false false)
  (return))

(fn `LightSetting`
  (`MaterialInstanceDynamic.SetScalarParameterValue` (`self.DM_body`) "FrontLight" (select `bool` (`self.Front`) :`true` 1.0))
  (`MaterialInstanceDynamic.SetScalarParameterValue` (`self.DM_body`) "RSideLight" (select `bool` (`self.Right`) :`true` 1.0))
  (`MaterialInstanceDynamic.SetScalarParameterValue` (`self.DM_body`) "LSideLight" (select `bool` (`self.Left`) :`true` 1.0))
  (`MaterialInstanceDynamic.SetScalarParameterValue` (`self.DM_body`) "BackLight" (select `bool` (`self.Back`) :`true` 1.0))
  (`MaterialInstanceDynamic.SetScalarParameterValue` (`self.DM_body`) "StopLight" (select `bool` (`self.Stop`) :`true` 1.0))
  (`MaterialInstanceDynamic.SetScalarParameterValue` (`self.DM_body`) "BotLight" (select `bool` (`self.Additional`) :`true` 1.0))
  (return))

(fn `MatrialsSetting`
  (bind _dm_body (`self.DM_body`))
  (bind _dm_body_2 (`self.DM_body`))
  (bind _dm_body_3 (`self.DM_body`))
  (bind _dm_body_4 (`self.DM_body`))
  (`MaterialInstanceDynamic.SetVectorParameterValue` _dm_body_3 "BaseColor" (`self.Color`))
  (`MaterialInstanceDynamic.SetVectorParameterValue` (`self.DM_topDetal`) "BaseColor" (`self.Color`))
  (`MaterialInstanceDynamic.SetScalarParameterValue` _dm_body_3 "BaseMetal" (`self.Metal`))
  (`MaterialInstanceDynamic.SetScalarParameterValue` (`self.DM_topDetal`) "BaseMetal" (`self.Metal`))
  (`MaterialInstanceDynamic.SetScalarParameterValue` _dm_body_3 "BaseSpecular" (`self.Specular`))
  (`MaterialInstanceDynamic.SetScalarParameterValue` (`self.DM_topDetal`) "BaseSpecular" (`self.Specular`))
  (`MaterialInstanceDynamic.SetScalarParameterValue` _dm_body_3 "BaseRoughness" (`self.Roughness`))
  (`MaterialInstanceDynamic.SetScalarParameterValue` (`self.DM_topDetal`) "BaseRoughness" (`self.Roughness`))
  (`MaterialInstanceDynamic.SetVectorParameterValue` _dm_body_3 "SecontColor" (`self.SecondColor`))
  (`MaterialInstanceDynamic.SetScalarParameterValue` _dm_body_3 "SecontMetal" (`self.SecondMetal`))
  (`MaterialInstanceDynamic.SetScalarParameterValue` _dm_body_3 "SecontRoughness" (`self.SecondRoughness`))
  (`MaterialInstanceDynamic.SetScalarParameterValue` _dm_body_3 "SecontSpecular" (`self.SecondSpecular`))
  (`MaterialInstanceDynamic.SetTextureParameterValue` _dm_body_3 "PaintColor" (select `/Game/ClassicBus1960/Blueprints/Enum/ENUM_ClassicBus1960_PaintType` (`self.PaintType`) :`NewEnumerator0` "/Game/ClassicBus1960/Textures/TX_ClassicBus1960_PaintMaskClean.TX_ClassicBus1960_PaintMaskClean" :`NewEnumerator1` "/Game/ClassicBus1960/Textures/TX_ClassicBus1960_PaintMask.TX_ClassicBus1960_PaintMask" :`NewEnumerator2` "/Game/ClassicBus1960/Textures/TX_ClassicBus1960_PaintMask1.TX_ClassicBus1960_PaintMask1" :`NewEnumerator3` "/Game/ClassicBus1960/Textures/TX_ClassicBus1960_PaintMask2.TX_ClassicBus1960_PaintMask2" :`NewEnumerator4` "/Game/ClassicBus1960/Textures/TX_ClassicBus1960_PaintMask3.TX_ClassicBus1960_PaintMask3" :!type "Texture Object Reference"))
  (`MaterialInstanceDynamic.SetVectorParameterValue` _dm_body "DirtColor" (`self.DirtColor`))
  (`MaterialInstanceDynamic.SetVectorParameterValue` (`self.DM_Inside`) "DirtColor" (`self.DirtColor`))
  (`MaterialInstanceDynamic.SetVectorParameterValue` (`self.DM_FWheel`) "DirtColor" (`self.DirtColor`))
  (`MaterialInstanceDynamic.SetVectorParameterValue` (`self.DM_BWheel`) "DirtColor" (`self.DirtColor`))
  (`MaterialInstanceDynamic.SetVectorParameterValue` (`self.DM_Under`) "DirtColor" (`self.DirtColor`))
  (`MaterialInstanceDynamic.SetVectorParameterValue` (`self.DM_topDetal`) "DirtColor" (`self.DirtColor`))
  (`MaterialInstanceDynamic.SetVectorParameterValue` (`self.DM_Curtain`) "DirtColor" (`self.DirtColor`))
  (`MaterialInstanceDynamic.SetScalarParameterValue` _dm_body "DirtSpecular" (`self.DirtSpecular`))
  (`MaterialInstanceDynamic.SetScalarParameterValue` (`self.DM_glass`) "DirtSpecular" (`self.DirtSpecular`))
  (`MaterialInstanceDynamic.SetScalarParameterValue` (`self.DM_Inside`) "DirtSpecular" (`self.DirtSpecular`))
  (`MaterialInstanceDynamic.SetScalarParameterValue` (`self.DM_FWheel`) "DirtSpecular" (`self.DirtSpecular`))
  (`MaterialInstanceDynamic.SetScalarParameterValue` (`self.DM_BWheel`) "DirtSpecular" (`self.DirtSpecular`))
  (`MaterialInstanceDynamic.SetScalarParameterValue` (`self.DM_Under`) "DirtSpecular" (`self.DirtSpecular`))
  (`MaterialInstanceDynamic.SetScalarParameterValue` (`self.DM_topDetal`) "DirtSpecular" (`self.DirtSpecular`))
  (`MaterialInstanceDynamic.SetScalarParameterValue` (`self.DM_Curtain`) "DirtSpecular" (`self.DirtSpecular`))
  (`MaterialInstanceDynamic.SetScalarParameterValue` _dm_body "DirtMetal" (`self.DirtMetal`))
  (`MaterialInstanceDynamic.SetScalarParameterValue` (`self.DM_glass`) "DirtMetal" (`self.DirtMetal`))
  (`MaterialInstanceDynamic.SetScalarParameterValue` (`self.DM_Inside`) "DirtMetal" (`self.DirtMetal`))
  (`MaterialInstanceDynamic.SetScalarParameterValue` (`self.DM_FWheel`) "DirtMetal" (`self.DirtMetal`))
  (`MaterialInstanceDynamic.SetScalarParameterValue` (`self.DM_BWheel`) "DirtMetal" (`self.DirtMetal`))
  (`MaterialInstanceDynamic.SetScalarParameterValue` (`self.DM_Under`) "DirtMetal" (`self.DirtMetal`))
  (`MaterialInstanceDynamic.SetScalarParameterValue` (`self.DM_topDetal`) "DirtMetal" (`self.DirtMetal`))
  (`MaterialInstanceDynamic.SetScalarParameterValue` (`self.DM_Curtain`) "DirtMetal" (`self.DirtMetal`))
  (`MaterialInstanceDynamic.SetScalarParameterValue` _dm_body "DirtRoughness" (`self.DirtRoughness`))
  (`MaterialInstanceDynamic.SetScalarParameterValue` (`self.DM_glass`) "DirtRoughness" (`self.DirtRoughness`))
  (`MaterialInstanceDynamic.SetScalarParameterValue` (`self.DM_Inside`) "DirtRoughness" (`self.DirtRoughness`))
  (`MaterialInstanceDynamic.SetScalarParameterValue` (`self.DM_FWheel`) "DirtRoughness" (`self.DirtRoughness`))
  (`MaterialInstanceDynamic.SetScalarParameterValue` (`self.DM_BWheel`) "DirtRoughness" (`self.DirtRoughness`))
  (`MaterialInstanceDynamic.SetScalarParameterValue` (`self.DM_Under`) "DirtRoughness" (`self.DirtRoughness`))
  (`MaterialInstanceDynamic.SetScalarParameterValue` (`self.DM_topDetal`) "DirtRoughness" (`self.DirtRoughness`))
  (`MaterialInstanceDynamic.SetScalarParameterValue` (`self.DM_Curtain`) "DirtRoughness" (`self.DirtRoughness`))
  (`MaterialInstanceDynamic.SetScalarParameterValue` _dm_body "DirtContrast" (`self.DirtContrast`))
  (`MaterialInstanceDynamic.SetScalarParameterValue` (`self.DM_glass`) "DirtContrast" (`self.DirtContrast`))
  (`MaterialInstanceDynamic.SetScalarParameterValue` (`self.DM_Inside`) "DirtContrast" (`self.DirtContrast`))
  (`MaterialInstanceDynamic.SetScalarParameterValue` (`self.DM_FWheel`) "DirtContrast" (`self.DirtContrast`))
  (`MaterialInstanceDynamic.SetScalarParameterValue` (`self.DM_BWheel`) "DirtContrast" (`self.DirtContrast`))
  (`MaterialInstanceDynamic.SetScalarParameterValue` (`self.DM_Under`) "DirtContrast" (`self.DirtContrast`))
  (`MaterialInstanceDynamic.SetScalarParameterValue` (`self.DM_topDetal`) "DirtContrast" (`self.DirtContrast`))
  (`MaterialInstanceDynamic.SetScalarParameterValue` (`self.DM_Curtain`) "DirtContrast" (`self.DirtContrast`))
  (`MaterialInstanceDynamic.SetScalarParameterValue` _dm_body "DirtIntence" (`self.Dirt`))
  (`MaterialInstanceDynamic.SetScalarParameterValue` (`self.DM_glass`) "DirtIntence" (`self.Dirt`))
  (`MaterialInstanceDynamic.SetScalarParameterValue` (`self.DM_Inside`) "DirtIntence" (`self.Dirt`))
  (`MaterialInstanceDynamic.SetScalarParameterValue` (`self.DM_FWheel`) "DirtIntence" (`self.Dirt`))
  (`MaterialInstanceDynamic.SetScalarParameterValue` (`self.DM_BWheel`) "DirtIntence" (`self.Dirt`))
  (`MaterialInstanceDynamic.SetScalarParameterValue` (`self.DM_Under`) "DirtIntence" (`self.Dirt`))
  (`MaterialInstanceDynamic.SetScalarParameterValue` (`self.DM_topDetal`) "DirtIntence" (`self.Dirt`))
  (`MaterialInstanceDynamic.SetScalarParameterValue` (`self.DM_Curtain`) "DirtIntence" (`self.Dirt`))
  (`MaterialInstanceDynamic.SetVectorParameterValue` (`self.DM_glass`) "DirtColor" (`self.DustColor`))
  (`MaterialInstanceDynamic.SetVectorParameterValue` (`self.DM_Curtain`) "Color" (`self.CurtainColor`))
  (`MaterialInstanceDynamic.SetScalarParameterValue` (`self.DM_glass`) "Wipers " (`self.Wipers `))
  (`MaterialInstanceDynamic.SetVectorParameterValue` _dm_body_2 "RustColor" (`self.RustColor`))
  (`MaterialInstanceDynamic.SetVectorParameterValue` (`self.DM_FWheel`) "RustColor" (`self.RustColor`))
  (`MaterialInstanceDynamic.SetVectorParameterValue` (`self.DM_BWheel`) "RustColor" (`self.RustColor`))
  (`MaterialInstanceDynamic.SetVectorParameterValue` (`self.DM_Under`) "RustColor" (`self.RustColor`))
  (`MaterialInstanceDynamic.SetScalarParameterValue` _dm_body_2 "RustSpecular" (`self.RustSpecular`))
  (`MaterialInstanceDynamic.SetScalarParameterValue` (`self.DM_FWheel`) "RustSpecular" (`self.RustSpecular`))
  (`MaterialInstanceDynamic.SetScalarParameterValue` (`self.DM_BWheel`) "RustSpecular" (`self.RustSpecular`))
  (`MaterialInstanceDynamic.SetScalarParameterValue` (`self.DM_Under`) "RustSpecular" (`self.RustSpecular`))
  (`MaterialInstanceDynamic.SetScalarParameterValue` _dm_body_2 "RustRoughness" (`self.RustRoughness`))
  (`MaterialInstanceDynamic.SetScalarParameterValue` (`self.DM_FWheel`) "RustRoughness" (`self.RustRoughness`))
  (`MaterialInstanceDynamic.SetScalarParameterValue` (`self.DM_BWheel`) "RustRoughness" (`self.RustRoughness`))
  (`MaterialInstanceDynamic.SetScalarParameterValue` (`self.DM_Under`) "RustRoughness" (`self.RustRoughness`))
  (`MaterialInstanceDynamic.SetScalarParameterValue` _dm_body_2 "RustMetal" (`self.RustMetal`))
  (`MaterialInstanceDynamic.SetScalarParameterValue` (`self.DM_FWheel`) "RustMetal" (`self.RustMetal`))
  (`MaterialInstanceDynamic.SetScalarParameterValue` (`self.DM_BWheel`) "RustMetal" (`self.RustMetal`))
  (`MaterialInstanceDynamic.SetScalarParameterValue` (`self.DM_Under`) "RustMetal" (`self.RustMetal`))
  (`MaterialInstanceDynamic.SetScalarParameterValue` _dm_body_2 "Rust" (`self.Rust`))
  (`MaterialInstanceDynamic.SetScalarParameterValue` (`self.DM_FWheel`) "Rust" (`self.Rust`))
  (`MaterialInstanceDynamic.SetScalarParameterValue` (`self.DM_BWheel`) "Rust" (`self.Rust`))
  (`MaterialInstanceDynamic.SetScalarParameterValue` (`self.DM_Under`) "Rust" (`self.Rust`))
  (`MaterialInstanceDynamic.SetScalarParameterValue` _dm_body_2 "RustContrast" (`self.RustContrast`))
  (`MaterialInstanceDynamic.SetScalarParameterValue` (`self.DM_FWheel`) "RustContrast" (`self.RustContrast`))
  (`MaterialInstanceDynamic.SetScalarParameterValue` (`self.DM_BWheel`) "RustContrast" (`self.RustContrast`))
  (`MaterialInstanceDynamic.SetScalarParameterValue` (`self.DM_Under`) "RustContrast" (`self.RustContrast`))
  (`MaterialInstanceDynamic.SetVectorParameterValue` _dm_body_4 "AttritionColor" (`self.AttritionColor`))
  (`MaterialInstanceDynamic.SetScalarParameterValue` _dm_body_4 "AttritonSpecular" (`self.AttritionSpecular`))
  (`MaterialInstanceDynamic.SetScalarParameterValue` _dm_body_4 "AttritionMetal" (`self.AttritionMetal`))
  (`MaterialInstanceDynamic.SetScalarParameterValue` _dm_body_4 "AttritionRoughness" (`self.AttritionRoughness`))
  (`MaterialInstanceDynamic.SetScalarParameterValue` _dm_body_4 "Attrition" (`self.Attrition`))
  (`MaterialInstanceDynamic.SetScalarParameterValue` _dm_body_4 "AttritionContrast" (`self.AttritionContrast`))
  (return))

(fn `UserConstructionScript`
  (`self.FDoorAction` (`self.FDoors`))
  (`self.BDoorAction` (`self.BDoors`))
  (`self.DetalsSetup`)
  (`self.CreateDynamicMat`)
  (`self.MatrialsSetting`)
  (`self.LightSetting`)
  (`self.WheelSetting`)
  (if (`self.WheelsSplit`)
    (`self.WheelsRotate`)))

(fn `WheelRoll`
  (`SceneComponent.K2_AddRelativeRotation` (`self.bw2`) (`KismetMathLibrary.MakeRotator` (`self.Roll`) (.pitch (`SceneComponent.RelativeRotation` (`self.bw1`))) (.yaw (`SceneComponent.RelativeRotation` (`self.bw1`)))) false false)
  (`SceneComponent.K2_AddRelativeRotation` (`self.fw1`) (`KismetMathLibrary.MakeRotator` (`self.Roll`) (.pitch (`SceneComponent.RelativeRotation` (`self.bw1`))) (.yaw (`SceneComponent.RelativeRotation` (`self.bw1`)))) false false)
  (`SceneComponent.K2_AddRelativeRotation` (`self.fw2`) (`KismetMathLibrary.MakeRotator` (`self.Roll`) (.pitch (`SceneComponent.RelativeRotation` (`self.bw1`))) (.yaw (`SceneComponent.RelativeRotation` (`self.bw1`)))) false false)
  (`SceneComponent.K2_AddRelativeRotation` (`self.bw1`) (`KismetMathLibrary.MakeRotator` (`self.Roll`) (.pitch (`SceneComponent.RelativeRotation` (`self.bw1`))) (.yaw (`SceneComponent.RelativeRotation` (`self.bw1`)))) false false)
  (return))

(fn `WheelSetting`
  (if (`self.WheelsSplit`)
    (`ActorComponent.K2_DestroyComponent` (`self.sm_Wheels`))
    (return)
    (else
      (`ActorComponent.K2_DestroyComponent` (`self.bw2`))
      (`ActorComponent.K2_DestroyComponent` (`self.bw1`))
      (`ActorComponent.K2_DestroyComponent` (`self.fw2`))
      (`ActorComponent.K2_DestroyComponent` (`self.fw1`))
      (return))))

(fn `WheelsRotate`
  (bind _fw1 (`self.fw1`))
  (`SceneComponent.K2_SetRelativeRotation` _fw1 (`KismetMathLibrary.MakeRotator` (.roll (`SceneComponent.RelativeRotation` _fw1)) (.pitch (`SceneComponent.RelativeRotation` _fw1)) (`self.Rotate`)) false false)
  (`SceneComponent.K2_SetRelativeRotation` (`self.fw2`) (`KismetMathLibrary.MakeRotator` (.roll (`SceneComponent.RelativeRotation` _fw1)) (.pitch (`SceneComponent.RelativeRotation` _fw1)) (`self.Rotate`)) false false)
  (return))